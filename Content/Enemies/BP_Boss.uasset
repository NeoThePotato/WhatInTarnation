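; BP_Boss is a burrowing boss that chases the player through the ground using a physics-driven skeletal mesh.
; Each tick, an upward trace from the head flags it as underground when it hits.
; While underground, force on the head bone pulls it toward the player, with velocity clamped.
; Dust and short-lived decals telegraph its position on the surface above, with decals growing as the head nears the surface.
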(event Game|Damage|EventAnyDamage
  (params (Damage :type Float%20%28single-precision%29) (DamageType :type Damage%20Type%20Object%20Reference) (InstigatedBy :type Controller%20Object%20Reference) (DamageCauser :type Actor%20Object%20Reference)))

(event EventTick
  (params (DeltaSeconds :type Float%20%28single-precision%29))
  (bind (_isunderground _groundpoint) (CallFunction|UpdateIsGrounded 1e+04))
  (CallFunction|UpdateTelegraphUnderground _groundpoint "400.000000,400.000000,400.000000")
  (if _isunderground
    (CallFunction|MoveTowardsPlayer)))

(event EventBeginPlay
  (Variables|Default|SetTarget (Game|GetPlayerCharacter 0)))

(fn ConstructionScript)

(fn UpdateIsGrounded
  (params (LineTraceLength :type Float%20%28double-precision%29))
  (bind _location (Utilities|GetHeadLocation))
  (bind (_outhit _returnvalue) (Collision|LineTraceByChannel _location (+ _location (Math|Vector|MakeVector 0.0 0.0 LineTraceLength)) "TraceTypeQuery1" false 0 "None"))
  (bind _output_get (Variables|Default|SetIsUnderground _returnvalue))
  (return _output_get _outhit))

(fn MoveTowardsPlayer
  (bind _headbone (Variables|Default|GetHeadBone))
  (bind _skeletalmesh (Variables|Default|GetSkeletalMesh))
  (Physics|AddForce _skeletalmesh (* (Math|Vector|Normalize (Math|Vector|GetUnitDirection(Vector) (Utilities|GetHeadLocation) (Transformation|GetActorLocation (Variables|Default|GetTarget)))) (Variables|Default|GetFollowSpeed)) _headbone true)
  (bind _returnvalue (Class|SkeletalMeshComponent|GetBoneLinearVelocity _skeletalmesh _headbone))
  (Physics|SetPhysicsLinearVelocity _skeletalmesh (Math|Vector|ClampVectorSize _returnvalue 1.0 (Variables|Default|GetMaxFollowVelocity)) false _headbone))

(fn UpdateTelegraphUnderground
  (params (GroundPoint :type Hit%20Result%20Structure) (DecalSize :type Vector :default "400.000000,400.000000,400.000000"))
  (bind (_bblockinghit _binitialoverlap _time _distance _location _impactpoint _normal _impactnormal _physmat _hitactor _hitcomponent) (Collision|BreakHitResult GroundPoint))
  (bind _isunderground (Variables|Default|GetIsUnderground))
  (bind _dust (Variables|Default|GetDust))
  (Rendering|SetVisibility _dust _isunderground false)
  (if _isunderground
    (Class|GameplayStatics|SpawnDecalAttached "/Game/Materials/M_Dust.M_Dust" (* (Math|Float|Clamp(Float) (Math|Float|Lerp 1.0 0.0 (/ _distance 1e+03)) 0.05) DecalSize) _hitcomponent "None" _location (Math|Conversions|RotationFromXVector _normal) "KeepWorldPosition" 2.0)
    (Transformation|SetWorldLocation _dust _location false false))
  (return))